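; Base zombie character Blueprint with health, melee attacks and ragdoll death.
; Attack sets a flag that an anim notify clears, while a damage notify hurts other actors overlapping the left and right damage spheres.
; Damage events reduce health and play sounds, then Die enables ragdoll physics and disables capsule collision, with Tick re-enabling physics if needed.
; The construction script snaps a sphere to the head socket.
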(event `self.ReceiveTick`
  (params (DeltaSeconds :type "Float (single-precision)"))
  (bind _mesh (`self.Mesh`))
  (if (and (not (`SceneComponent.IsSimulatingPhysics` _mesh "None")) (`self.Dead`))
    (`PrimitiveComponent.SetSimulatePhysics` _mesh true)))

(event `self.ReceiveAnyDamage`
  (params (Damage :type "Float (single-precision)") (DamageType :type "DamageType Object Reference") (InstigatedBy :type "Controller Object Reference") (DamageCauser :type "Actor Object Reference"))
  (if (not (`self.Dead`))
    (bind _output_get (set `self.Health` (- (`self.Health`) Damage)))
    (`GameplayStatics.PlaySoundAtLocation` (`self.HurtSound`) (`self.K2_GetActorLocation`) (struct) 1.0 1.0 0.0 null null null)
    (if (<= _output_get 0.0)
      (`self.Die`))))

(event `self.ReceivePointDamage`
  (params (Damage :type "Float (single-precision)") (DamageType :type "DamageType Object Reference") (HitLocation :type "Vector Structure") (HitNormal :type "Vector Structure") (HitComponent :type "PrimitiveComponent Object Reference") (BoneName :type Name) (ShotFromDirection :type "Vector Structure") (InstigatedBy :type "Controller Object Reference") (DamageCauser :type "Actor Object Reference") (HitInfo :type "HitResult Structure (by ref)"))
  (if (not (`self.Dead`))
    (bind _output_get (set `self.Health` (- (`self.Health`) 1.0)))
    (`GameplayStatics.PlaySoundAtLocation` (`self.HurtSound`) (`self.K2_GetActorLocation`) (struct) 1.0 1.0 0.0 null null null)
    (if (<= _output_get 0.0)
      (`self.Die`))))

(fn `AnimNotify_Damage`
  (for _array_element (`PrimitiveComponent.GetOverlappingActors` (`self.DamageSphereRight`) "/Script/Engine.Actor")
    (if (!= _array_element self)
      (`GameplayStatics.ApplyDamage` _array_element (`self.Damage`) null self "/Game/ShooterAI/WeaponSystem/DamageTypes/BPD_PointDamage.BPD_PointDamage_C")))
  (for _array_element_2 (`PrimitiveComponent.GetOverlappingActors` (`self.DamageSphereLeft`) "/Script/Engine.Actor")
    (if (!= _array_element_2 self)
      (`GameplayStatics.ApplyDamage` _array_element_2 (`self.Damage`) null self "/Game/ShooterAI/WeaponSystem/DamageTypes/BPD_PointDamage.BPD_PointDamage_C"))))

(fn `AnimNotify_EndAttack`
  (set `self.Attacking` false))

(fn `Attack`
  (params (TargetLocation :type "Vector Structure"))
  (returns (Success :type Boolean))
  (bind _output_get (set `self.Attacking` true))
  (return _output_get))

(fn `Die`
  (bind _mesh (`self.Mesh`))
  (`SkeletalMeshComponent.SetAnimationMode` _mesh "AnimationCustomMode")
  (`PrimitiveComponent.SetSimulatePhysics` _mesh true)
  (set `self.Dead` true)
  (`GameplayStatics.PlaySoundAtLocation` (`self.DeathSound`) (`self.K2_GetActorLocation`) (struct) 1.0 1.0 0.0 null null null)
  (`PrimitiveComponent.SetCollisionEnabled` (`self.CapsuleComponent`) "NoCollision"))

(fn `UserConstructionScript`
  (`SceneComponent.K2_AttachToComponent` (`self.Sphere`) (`self.Mesh`) (`self.HeadBoneSocket`) "SnapToTarget" "KeepRelative" "KeepRelative" true))