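; Base Blueprint for headcrab AI enemies, providing death handling and a placeholder jump attack.
; Die switches the mesh to custom animation mode, enables physics simulation, sets the Dead flag and plays the death sound at the actor's location.
; Tick re-enables mesh physics whenever a dead headcrab is not simulating.
; JumpAttack takes a target location but only returns false, with no attack logic here.
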(event `self.ReceiveTick`
  (params (DeltaSeconds :type "Float (single-precision)"))
  (bind _mesh (`self.Mesh`))
  (if (and (not (`SceneComponent.IsSimulatingPhysics` _mesh "None")) (`self.Dead`))
    (`PrimitiveComponent.SetSimulatePhysics` _mesh true)))

(fn `Die`
  (bind _mesh (`self.Mesh`))
  (`SkeletalMeshComponent.SetAnimationMode` _mesh "AnimationCustomMode")
  (`PrimitiveComponent.SetSimulatePhysics` _mesh true)
  (set `self.Dead` true)
  (`GameplayStatics.PlaySoundAtLocation` (`self.DeathSound`) (`self.K2_GetActorLocation`) (struct) 1.0 1.0 0.0 null null null))

(fn `JumpAttack`
  (params (TargetLocation :type "Vector Structure"))
  (returns (Success :type Boolean))
  (return false))

(fn `UserConstructionScript`)