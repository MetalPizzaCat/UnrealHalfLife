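; Classic headcrab enemy that leaps at targets, hurts nearby non-headcrab actors and can be killed.
; JumpAttack jumps toward a location, applies damage to DamageSphere overlaps, then Tick clears the attack lock after a cooldown.
; The attack notify plays the jump montage; BeUsed calls JumpAttack and plays it only on a false return.
; Damage events reduce health until Die, and Tick later switches the dead mesh to physics simulation.
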(event `self.ReceiveBeginPlay`
  (add `self.NotifyAttack` (delegate `NotifyAttack_Event`)))

(event `NotifyAttack_Event`
  (bind _mesh (`self.Mesh`))
  (`|PlayMontage` _mesh "/Game/hl2/headcrab_classic/headcrab_classic_Anim_headcrabclassic_qc_skeleton_jumpattack_broadcast_Montage.headcrab_classic_Anim_headcrabclassic_qc_skeleton_jumpattack_broadcast_Montage"
    (:`OnCompleted`
      (`SkeletalMeshComponent.SetAnimationMode` _mesh "AnimationBlueprint"))))

(event `self.ReceiveTick`
  (params (DeltaSeconds :type "Float (single-precision)"))
  (bind _mesh (`self.Mesh`))
  (bind _output_get (set `self.TimeSinceLastAttack` (+ DeltaSeconds (`self.TimeSinceLastAttack`))))
  (if (>= _output_get 1.5)
    (set `self.Attacking` false)
    (if (and (not (`SceneComponent.IsSimulatingPhysics` _mesh "None")) (`self.Dead`))
      (`PrimitiveComponent.SetSimulatePhysics` _mesh true))))

(event `self.BeUsed`
  (params (user :type "Actor Object Reference"))
  (bind _mesh (`self.Mesh`))
  (bind _success (`self.JumpAttack` (`self.K2_GetActorLocation` user)))
  (if (not _success)
    (`|PlayMontage` _mesh "/Game/hl2/headcrab_classic/headcrab_classic_Anim_headcrabclassic_qc_skeleton_jumpattack_broadcast_Montage.headcrab_classic_Anim_headcrabclassic_qc_skeleton_jumpattack_broadcast_Montage"
      (:`OnCompleted`
        (`SkeletalMeshComponent.SetAnimationMode` _mesh "AnimationBlueprint")))))

(event `self.ReceiveAnyDamage`
  (params (Damage :type "Float (single-precision)") (DamageType :type "DamageType Object Reference") (InstigatedBy :type "Controller Object Reference") (DamageCauser :type "Actor Object Reference"))
  (if (not (`self.Dead`))
    (bind _output_get (set `self.Health` (- (`self.Health`) Damage)))
    (`GameplayStatics.PlaySoundAtLocation` (`self.HurtSound`) (`self.K2_GetActorLocation`) (struct) 1.0 1.0 0.0 null null null)
    (if (<= _output_get 0.0)
      (`self.Die`))))

(event `self.ReceivePointDamage`
  (params (Damage :type "Float (single-precision)") (DamageType :type "DamageType Object Reference") (HitLocation :type "Vector Structure") (HitNormal :type "Vector Structure") (HitComponent :type "PrimitiveComponent Object Reference") (BoneName :type Name) (ShotFromDirection :type "Vector Structure") (InstigatedBy :type "Controller Object Reference") (DamageCauser :type "Actor Object Reference") (HitInfo :type "HitResult Structure (by ref)"))
  (if (not (`self.Dead`))
    (bind _output_get (set `self.Health` (- (`self.Health`) 1.0)))
    (`GameplayStatics.PlaySoundAtLocation` (`self.HurtSound`) (`self.K2_GetActorLocation`) (struct) 1.0 1.0 0.0 null null null)
    (if (<= _output_get 0.0)
      (`self.Die`))))

(fn `JumpAttack`
  (params (TargetLocation :type "Vector Structure"))
  (returns (Success :type Boolean))
  (if (not (`self.Attacking`))
    (if (not (`self.Dead`))
      (`self.Jump`)
      (`self.AddMovementInput` (`KismetMathLibrary.GetForwardVector` (`KismetMathLibrary.FindLookAtRotation` (`self.K2_GetActorLocation`) TargetLocation)) 100.0)
      (for _array_element (`PrimitiveComponent.GetOverlappingActors` (`self.DamageSphere`) "/Script/Engine.Actor")
        (if (!= _array_element self)
          (cast `/Game/AI/Headcrab/BP_HeadcrabBase` _array_element ; Headcrab can not damage other head crabs
            (:`CastFailed`
              (`GameplayStatics.ApplyDamage` _array_element (`self.Damage`) null null "/Game/ShooterAI/WeaponSystem/DamageTypes/BPD_PointDamage.BPD_PointDamage_C")))))
      (set `self.Attacking` true)
      (set `self.TimeSinceLastAttack` 0.0)
      (return true)
      (else
        (return false)))))

(fn `UserConstructionScript`)