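; AI node system actor that marks an area for AI pawns to search, using a trigger sphere sized by Radius.
; On overlap, a new pawn whose condition message matches ConditionsWhenAreaShouldBeSearched receives this actor as a temporary patrol, starting at the first node.
; Searchers tracks those pawns to avoid repeat assignment and drops them on end overlap.
; A closest-node selection loop exists but is disconnected.
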(event `self.Sphere.OnComponentBeginOverlap`
  (params (OverlappedComponent :type "PrimitiveComponent Object Reference") (OtherActor :type "Actor Object Reference") (OtherComp :type "PrimitiveComponent Object Reference") (OtherBodyIndex :type Integer) (bFromSweep :type Boolean) (SweepResult :type "HitResult Structure (by ref)"))
  (if (== (`KismetArrayLibrary.Array_Find` (`self.Searchers`) OtherActor) -1)
    (bind _condition (message `/Game/ShooterAI/Blueprints/BPI_ShooterAI.GetPawnCondition` OtherActor))
    (for _array_element (`self.ConditionsWhenAreaShouldBeSearched`)
      (if (`|EnumEquality` _condition _array_element)
        (set `self.Should` true)
        (break)))
    (if (`self.Should`)
      (message `/Game/ShooterAI/Blueprints/BPI_ShooterAI.SetTempAIPatrol` OtherActor self (`|GetArrayItem` (`self.Nodes`)) -1)
      (`KismetArrayLibrary.Array_Add` (`self.Searchers`) OtherActor))))

(event `self.Sphere.OnComponentEndOverlap`
  (params (OverlappedComponent :type "PrimitiveComponent Object Reference") (OtherActor :type "Actor Object Reference") (OtherComp :type "PrimitiveComponent Object Reference") (OtherBodyIndex :type Integer))
  (bind _searchers (`self.Searchers`))
  (`KismetArrayLibrary.Array_Remove` _searchers (`KismetArrayLibrary.Array_Find` _searchers OtherActor)))

(fn `UserConstructionScript`
  (`parent.UserConstructionScript`)
  (`SphereComponent.SetSphereRadius` (`self.Sphere`) (`self.Radius`) true))