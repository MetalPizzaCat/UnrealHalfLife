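; Sniper AI controller that starts the BT_SolderSniper behavior tree and turns sight perception into combat state.
; UpdateSenseSight checks for dead friendlies near the pawn and, depending on its stress reaction, changes Condition.
; Without an enemy, it picks the first perceived character with a matching Relationships entry and writes it to the blackboard.
; When sight of the enemy is lost, it stores the last seen location and clears Enemy.
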(event `self.ReceiveBeginPlay`
  ;[1 0 0.8061] Default
  (`self.RunBehaviorTree` "/Game/ShooterAI/Blueprints/BT_SolderSniper.BT_SolderSniper"))

(event `self.UpdateSenseSight`
  (bind _returnvalue (`self.K2_GetPawn`))
  (bind _returnvalue_2 (`AIBlueprintHelperLibrary.GetBlackboard` null))
  (bind _returnvalue_3 (`AIBlueprintHelperLibrary.GetBlackboard` self))
  ;[0 0.005 0.995] Is there any dead friends anywhere close?
  (for _array_element (`AIPerceptionComponent.GetPerceivedActors` (`self.AIPerception`) "/Script/AIModule.AISense_Sight")
    (bind _aspawn (castclass `Pawn` (`GameplayStatics.GetObjectClass` _array_element)))
    (if (!= (`KismetArrayLibrary.Array_Find` (`self.FriendlyClasses`) _aspawn) -1)
      (bind _dead (message `/Game/ShooterAI/Blueprints/BPI_ShooterAI.GetIsDead` _array_element))
      (if _dead
        (if (<= (`KismetMathLibrary.VSize` (- (`self.K2_GetActorLocation` _array_element) (`self.K2_GetActorLocation` _returnvalue))) 300.0)
          (bind _reaction (message `/Game/ShooterAI/Blueprints/BPI_ShooterAI.PawnGetStressReaction` _returnvalue))
          (if (`|EnumEquality` _reaction "NewEnumerator0")
            (set `self.Condition` "NewEnumerator2"))))))
  (`/Engine/EditorBlueprintResources/StandardMacros.IsValid` (`BlackboardComponent.GetValueAsObject` _returnvalue_3 "Enemy")
    (:`Is Valid`
      ;[0 0 1 1 12] We loast enemy and going search last place where we saw it
      (if (not (`self.CanSeeTarget` (`BlackboardComponent.GetValueAsObject` (`AIBlueprintHelperLibrary.GetBlackboard` null) "Enemy")))
        (bind (_wasseen _location) (`self.GetLastSeenLocationOfTheObject` null))
        (`BlackboardComponent.SetValueAsVector` _returnvalue_2 "LastSeenLocationOfTheTarget" _location)
        (`BlackboardComponent.ClearValue` _returnvalue_2 "Enemy")))
    (:`Is Not Valid`
      ;[1 0.8786 0 1 10] Can see Enemy?
      (for _array_element_2 (`AIPerceptionComponent.GetPerceivedActors` (`self.AIPerception`) "/Script/AIModule.AISense_Sight")
        (bind _ascharacter (cast `Character` _array_element_2))
        (bind (_value _returnvalue_4) (`BlueprintMapLibrary.Map_Find` (`self.Relationships`) (`GameplayStatics.GetObjectClass` _ascharacter)))
        (if _returnvalue_4
          (if (`|EnumEquality` _value "NewEnumerator0")
            (`BlackboardComponent.SetValueAsObject` _returnvalue_3 "Enemy" _array_element_2)
            (`BlackboardComponent.SetValueAsBool` _returnvalue_3 "WasTargetSeen" true)
            (`BlackboardComponent.SetValueAsBool` _returnvalue_3 "IsEnemyTooFarAway" false)
            (break)))))))

(fn `UserConstructionScript`
  (`parent.UserConstructionScript`))