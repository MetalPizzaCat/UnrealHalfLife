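; Spawner actor that creates a batch of AI soldiers from a configurable pawn class and behavior tree.
; SpawnObjectEvent loops from 1 to Amount, using the loop index to pick each spawn offset relative to the actor.
; It can send each pawn an actor-relative stimulus location to go to via a message.
; Spawned BPAI_Solder pawns with a valid current weapon get their reserve and clip ammo overridden.
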(event `self.SpawnObject_Event`
  (for _index (range 1 (+ (`self.Amount`) 1))
    (bind _returnvalue (`AIBlueprintHelperLibrary.SpawnAIFromClass` (`self.Class`) (`self.BehaviourTree`) (+ (`|GetArrayItem` (`self.LocationsToSpawn`) _index) (`self.K2_GetActorLocation`))))
    (if (`self.HasLocationToBe`)
      (message `/Game/ShooterAI/Blueprints/BPI_ShooterAI.PawnSetStimulusLocation` _returnvalue (+ (`self.LocationToBe`) (`self.K2_GetActorLocation`))))
    (bind _asbpai_solder (cast `/Game/ShooterAI/Blueprints/BPAI_Solder` _returnvalue))
    (bind _currentweapon (`/Game/ShooterAI/Blueprints/BPAI_Solder.CurrentWeapon` _asbpai_solder))
    (`/Engine/EditorBlueprintResources/StandardMacros.IsValid` _currentweapon
      (:`Is Valid`
        (set `/Game/ShooterAI/WeaponSystem/BPA_WeaponBase.PrimaryAmountOfAmmo` (`self.AmountOfAmmo`) _currentweapon)
        (set `/Game/ShooterAI/WeaponSystem/BPA_WeaponBase.PrimaryAmmoInTheClip` (`self.AmmoInTheClip`) _currentweapon)))))

(fn `UserConstructionScript`
  (`parent.UserConstructionScript`))