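; BPA_Spawner is an actor that spawns a batch of AI pawns when its SpawnObject_Event is called.
; It loops from 1 to Amount, spawning the configured class with a behavior tree at LocationsToSpawn offsets from the actor's location, indexed by the loop counter.
; If HasLocationToBe is set, it messages each pawn with a stimulus location, also offset from the spawner.
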(event `SpawnObject_Event`
  (for _index (range 1 (+ (`self.Amount`) 1))
    (bind _returnvalue (`AIBlueprintHelperLibrary.SpawnAIFromClass` (`self.Class`) (`self.BehaviourTree`) (+ (`|GetArrayItem` (`self.LocationsToSpawn`) _index) (`self.K2_GetActorLocation`))))
    (if (`self.HasLocationToBe`)
      (message `/Game/ShooterAI/Blueprints/BPI_ShooterAI.PawnSetStimulusLocation` _returnvalue (+ (`self.LocationToBe`) (`self.K2_GetActorLocation`))))))

(fn `UserConstructionScript`)