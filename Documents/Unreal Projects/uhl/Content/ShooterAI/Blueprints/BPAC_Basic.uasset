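; Basic AI controller for shooter soldiers that runs BT_Solder and feeds its blackboard.
; Perception updates use the pawn's class relationship map to pick or drop living enemies by sight, flag their range and record noise locations.
; Low health, checked every tick, or nearby dead friendlies can change the Condition key.
; Interface messages share target contacts, forward damage locations to the pawn and assign patrol systems.
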(event `self.ReceiveTick`
  (params (DeltaSeconds :type "Float (single-precision)"))
  (`self.UpdateCondition`))

(event `self.ReceiveBeginPlay`
  (`self.RunBehaviorTree` "/Game/ShooterAI/Blueprints/BT_Solder.BT_Solder")
  (bind _system (message `/Game/ShooterAI/Blueprints/BPI_ShooterAI.PawnGetAIPatrolSystem` (`self.K2_GetPawn`)))
  (`BlackboardComponent.SetValueAsObject` (`AIBlueprintHelperLibrary.GetBlackboard` self) "PatrolSystem" _system))

(event `self.AIPerception.OnPerceptionUpdated`
  (params (UpdatedActors :type "Array of Actor Object Reference (by ref)"))
  (bind _returnvalue (`AIBlueprintHelperLibrary.GetBlackboard` null))
  (bind _returnvalue_2 (`self.K2_GetPawn`))
  (bind _ascharacter (cast `Character` (`self.K2_GetPawn`)))
  (bind (_classes _realationships) (message `/Game/ShooterAI/Blueprints/BPI_ShooterAI.GetClassRelationshipMap` _ascharacter))
  (for (_array_element _array_index) _classes
    (`BlueprintMapLibrary.Map_Add` (`self.Relationships`) _array_element (`|GetArrayItem` _realationships _array_index))
    (`self.UpdateSenseSight`)
    (`self.UpdateSenseHearing`)
    (`self.UpdateCondition`)
    (bind _dead (message `/Game/ShooterAI/Blueprints/BPI_ShooterAI.GetIsDead` _returnvalue_2))
    (`BlackboardComponent.SetValueAsBool` _returnvalue "Alive" (not _dead))
    (bind _spot (message `/Game/ShooterAI/Blueprints/BPI_ShooterAI.PawnGetSafeSpot` _returnvalue_2))
    (`BlackboardComponent.SetValueAsObject` _returnvalue "SafeSpot" _spot)))

(event `/Game/ShooterAI/Blueprints/BPI_ShooterAI.SetCondition`
  (params (Condition :type "/Game/ShooterAI/Blueprints/E_AICondition Enum" :default "NewEnumerator0"))
  (bind _output_get (set `self.Condition` Condition))
  (`BlackboardComponent.SetValueAsEnum` (`AIBlueprintHelperLibrary.GetBlackboard` null) "Condition" _output_get))

(event `/Game/ShooterAI/Blueprints/BPI_ShooterAI.ForceToSeeEnemy`
  (params (`Force?` :type Boolean))
  (set `self.ForcedToSeeEnemy` `Force?`))

(fn `AI_ControllerGetClosestNode`
  (params (PatrolSystem :type "/Game/ShooterAI/Blueprints/AINodeSystem/BPAN_Patrol Object Reference") (MaxDistance :type "Float (double-precision)"))
  (returns (Node :type "/Game/ShooterAI/Blueprints/AINodeSystem/BPAN_PatrolNode Object Reference"))
  (bind _node (`self.GetClosestPatrolNode` PatrolSystem MaxDistance))
  (return _node))

(fn `CanSeeTarget`
  (params (Object :type "Object Object Reference"))
  (returns (CanSee :type Boolean))
  (locals (Result :type Boolean))
  (for _array_element (`AIPerceptionComponent.GetCurrentlyPerceivedActors` (`self.AIPerception`) "/Script/AIModule.AISense_Sight")
    (bind _output_get (set `local.Result` (== _array_element Object)))
    (if _output_get
      (break)))
  (return (`local.Result`)))

(fn `GetCharacterIsplayingAnimation`
  (returns (is :type Boolean))
  (return false))

(fn `GetCharacterMesh`
  (returns (Mesh :type "SkeletalMeshComponent Object Reference"))
  (return null))

(fn `GetClassRelationshipMap`
  (returns (Classes :type "Array of Character Class Reference") (Realationships :type "Array of /Game/ShooterAI/Blueprints/E_RealationShip Enum"))
  (return))

(fn `GetClosestPatrolNode`
  (params (PatrolSystem :type "/Game/ShooterAI/Blueprints/AINodeSystem/BPAN_Patrol Object Reference") (MaxDistance :type "Float (double-precision)"))
  (returns (Node :type "/Game/ShooterAI/Blueprints/AINodeSystem/BPAN_PatrolNode Object Reference"))
  (locals (IndexOfResult :type Integer))
  (bind _nodes (`/Game/ShooterAI/Blueprints/AINodeSystem/BPAN_Patrol.Nodes` PatrolSystem))
  (for (_array_element _array_index) _nodes
    (if (<= (`KismetMathLibrary.VSize` (- (`self.K2_GetActorLocation` _array_element) (`self.K2_GetActorLocation` (`self.K2_GetPawn`)))) MaxDistance)
      (set `local.IndexOfResult` _array_index)
      (break)))
  (return (`|GetArrayItem` _nodes (`local.IndexOfResult`))))

(fn `GetDistanceToTarget`
  (params (Actor :type "Actor Object Reference"))
  (returns (Distance :type "Float (double-precision)"))
  (return (`KismetMathLibrary.VSize` (- (`self.K2_GetActorLocation` Actor) (`self.K2_GetActorLocation` (`self.K2_GetPawn`))))))

(fn `GetHealth`
  (returns (Health :type "Float (double-precision)"))
  (return 0.0))

(fn `GetIsCrouching`
  (returns (Is :type Boolean))
  (return false))

(fn `GetIsDead`
  (returns (Dead :type Boolean))
  (return false))

(fn `GetIsJumping`
  (returns (Is :type Boolean))
  (return false))

(fn `GetIsScoped`
  (returns (Is :type Boolean))
  (return false))

(fn `GetIsShooting`
  (returns (Is :type Boolean))
  (return false))

(fn `GetIsSprinting`
  (returns (Is :type Boolean))
  (return false))

(fn `GetLastSeenLocationOfTheObject`
  (params (Object :type "Object Object Reference"))
  (returns (WasSeen :type Boolean) (Location :type "Vector Structure"))
  (locals (Seen :type Boolean))
  (bind _aiperception (`self.AIPerception`))
  (bind _asactor (cast `Actor` Object)
    (:`then`
      (for _array_element (`AIPerceptionComponent.GetKnownPerceivedActors` _aiperception "/Script/AIModule.AISense_Sight")
        (if (== _array_element _asactor)
          (set `local.Seen` true)
          (break)))
      ;[0.03127 1 0] Get last location
      (if (`local.Seen`)
        (`AIPerceptionComponent.GetActorsPerception` _aiperception _asactor)
        (return (`local.Seen`) (`self.K2_GetActorLocation` _asactor))))
    (:`CastFailed`
      ;[1 0 0] Object isn't actor
      (return false (1.0 0.0 0.0)))))

(fn `GetLastStimulusLocation`
  (returns (Location :type "Vector Structure"))
  (bind _laststimuluslocation (`self.LastStimulusLocation`))
  (if (!= _laststimuluslocation (0.0 0.0 0.0) :`ErrorTolerance` 0.1)
    (`KismetSystemLibrary.PrintString` (`KismetStringLibrary.Conv_VectorToString` _laststimuluslocation))
    (return _laststimuluslocation)))

(fn `GetLastTargetLocation`
  (returns (Location :type "Vector Structure"))
  (return (`self.LastStimulusLocation`)))

(fn `GetMainMesh`
  (returns (Mesh :type "SkeletalMeshComponent Object Reference"))
  (return null))

(fn `GetPawnCondition`
  (returns (Condition :type "/Game/ShooterAI/Blueprints/E_AICondition Enum"))
  (return "NewEnumerator0"))

(fn `GetPawnPitchAndYaw`
  (returns (Pitch :type "Float (double-precision)") (Yaw :type "Float (double-precision)"))
  (return 0.0 0.0))

(fn `GetSpeedAndDirection`
  (returns (Speed :type "Float (double-precision)") (Direction :type "Float (double-precision)"))
  (return 0.0 0.0))

(fn `GetTargetIsInRange`
  (params (Range :type "Float (double-precision)") (Target :type "Actor Object Reference"))
  (returns (Result :type Boolean))
  (bind _distance (message `/Game/ShooterAI/Blueprints/BPI_ShooterAI.PawnGetMaxViewEnemyDistance` (`self.K2_GetPawn`)))
  (return (<= (`self.GetDistanceToTarget` Target) _distance)))

(fn `PawnCheckSurroundings`
  (returns (WasTargetFound :type Boolean))
  (return false))

(fn `PawnGetAIPatrolSystem`
  (returns (System :type "/Game/ShooterAI/Blueprints/AINodeSystem/BPAN_Patrol Object Reference"))
  (return null))

(fn `PawnGetMaxViewEnemyDistance`
  (returns (Distance :type "Float (double-precision)"))
  (return 0.0))

(fn `PawnGetSafeSpot`
  (returns (Spot :type "/Game/ShooterAI/Blueprints/AINodeSystem/BPAN_SafeLocation Object Reference"))
  (return null))

(fn `PawnGetStressReaction`
  (returns (Reaction :type "/Game/ShooterAI/Blueprints/E_StressReact Enum"))
  (return "NewEnumerator1"))

(fn `PawnGetTargetWasReached`
  (returns (Result :type Boolean))
  (return false))

(fn `PawnSayMessage`
  (params (BaseMessage :type "/Game/ShooterAI/Blueprints/BPS_AIMessage Structure") (MessageType :type "/Game/ShooterAI/Blueprints/AIMessageSystem/BPAM_Object Class Reference"))
  (returns (Success :type Boolean))
  (return false))

(fn `PickUpItem`
  (params (Item :type "StaticMesh Object Reference"))
  (returns (PickedUp :type Boolean))
  (return false))

(fn `ReceiveMessage`
  (params (Message :type "/Game/ShooterAI/Blueprints/AIMessageSystem/BPAM_Object Object Reference"))
  (returns (Success :type Boolean))
  (bind _returnvalue (`self.K2_GetPawn`))
  (bind _returnvalue_2 (`AIBlueprintHelperLibrary.GetBlackboard` null))
  (bind _asbpam_contact_with_target (cast `/Game/ShooterAI/Blueprints/AIMessageSystem/BPAM_ContactWithTarget` Message)
    (:`then`
      (bind _target (`/Game/ShooterAI/Blueprints/AIMessageSystem/BPAM_ContactWithTarget.Target` _asbpam_contact_with_target))
      (bind _asactor (cast `Actor` _target))
      (bind _distance (message `/Game/ShooterAI/Blueprints/BPI_ShooterAI.PawnGetMaxViewEnemyDistance` _returnvalue))
      (bind _returnvalue_3 (`self.K2_GetActorLocation` _asactor))
      (if (not (<= (`KismetMathLibrary.VSize` (- _returnvalue_3 (`self.K2_GetActorLocation` _returnvalue))) _distance))
        (bind _output_get (set `self.LastStimulusLocation` _returnvalue_3))
        (`BlackboardComponent.SetValueAsVector` _returnvalue_2 "LastStimulusLocation" _output_get))
      (`BlackboardComponent.SetValueAsObject` _returnvalue_2 "Enemy" _target)
      (return true))
    (:`CastFailed`
      (bind _asbpam_receiving_damage (cast `/Game/ShooterAI/Blueprints/AIMessageSystem/BPAM_ReceivingDamage` Message)
        (:`then`
          (message `/Game/ShooterAI/Blueprints/BPI_ShooterAI.PawnSetStimulusLocation` (`self.K2_GetPawn`) (`/Game/ShooterAI/Blueprints/AIMessageSystem/BPAM_ReceivingDamage.Where` _asbpam_receiving_damage)))
        (:`CastFailed`
          ;[1 0 0] Add here reaction that you want
          (cast `/Game/ShooterAI/Blueprints/AIMessageSystem/BPAM_SomethingSuspisious` Message))))))

(fn `StartSearchPatrol`
  (params (Patrol :type "/Game/ShooterAI/Blueprints/AINodeSystem/BPAN_Patrol Object Reference"))
  (returns (WasChaged :type Boolean))
  (`BlackboardComponent.SetValueAsObject` (`AIBlueprintHelperLibrary.GetBlackboard` null) "PatrolSystem" Patrol)
  (return true))

(fn `UpdateCondition`
  (bind _health (message `/Game/ShooterAI/Blueprints/BPI_ShooterAI.GetHealth` (`self.K2_GetPawn`)))
  (if (<= _health 20.0)
    (set `self.Condition` "NewEnumerator2"))
  (`BlackboardComponent.SetValueAsEnum` (`AIBlueprintHelperLibrary.GetBlackboard` null) "Condition" (`self.Condition`)))

(fn `UpdateSenseHearing`
  ;[0.9973 0.016 0.031] PLACE YOUR OWN WAY OF CHECKING IF PAWN SHOULD REACT TO NOISES
  (for _array_element (`AIPerceptionComponent.GetCurrentlyPerceivedActors` (`self.AIPerception`) "/Script/AIModule.AISense_Hearing")
    (castclass `/Game/ShooterAI/Blueprints/BPAI_Solder` (`GameplayStatics.GetObjectClass` _array_element)
      (:`CastFailed`
        (bind _output_get (set `self.LastStimulusLocation` (`self.K2_GetActorLocation` _array_element)))
        (`BlackboardComponent.SetValueAsVector` (`AIBlueprintHelperLibrary.GetBlackboard` null) "LastStimulusLocation" _output_get)
        (break)))))

(fn `UpdateSenseSight`
  (bind _returnvalue (`self.K2_GetPawn`))
  (bind _returnvalue_2 (`self.K2_GetPawn`))
  (bind _returnvalue_3 (`AIBlueprintHelperLibrary.GetBlackboard` null))
  (bind _returnvalue_4 (`self.K2_GetPawn`))
  (bind _returnvalue_5 (`AIBlueprintHelperLibrary.GetBlackboard` null))
  (bind _returnvalue_6 (`BlackboardComponent.GetValueAsObject` (`AIBlueprintHelperLibrary.GetBlackboard` null) "Enemy"))
  (bind _returnvalue_7 (`BlackboardComponent.GetValueAsObject` _returnvalue_3 "Enemy"))
  ;[0 0.005 0.995] Is there any dead friends anywhere close?
  (for _array_element (`AIPerceptionComponent.GetPerceivedActors` (`self.AIPerception`) "/Script/AIModule.AISense_Sight")
    (bind _aspawn (castclass `Pawn` (`GameplayStatics.GetObjectClass` _array_element)))
    (if (!= (`KismetArrayLibrary.Array_Find` (`self.FriendlyClasses`) _aspawn) -1)
      (bind _dead (message `/Game/ShooterAI/Blueprints/BPI_ShooterAI.GetIsDead` _array_element))
      (if _dead
        (if (<= (`KismetMathLibrary.VSize` (- (`self.K2_GetActorLocation` _array_element) (`self.K2_GetActorLocation` _returnvalue))) 300.0)
          (bind _reaction (message `/Game/ShooterAI/Blueprints/BPI_ShooterAI.PawnGetStressReaction` _returnvalue))
          (if (`|EnumEquality` _reaction "NewEnumerator0")
            (set `self.Condition` "NewEnumerator2"))))))
  (if (`self.ForcedToSeeEnemy`)
    (`BlackboardComponent.SetValueAsBool` (`AIBlueprintHelperLibrary.GetBlackboard` null) "IsEnemyTooFarAway" false)
    (else
      (`/Engine/EditorBlueprintResources/StandardMacros.IsValid` _returnvalue_7
        (:`Is Valid`
          ;[0 0 1 1 12] We loast enemy and going search last place where we saw it
          (if (`self.CanSeeTarget` _returnvalue_6)
            ;[0 1 0.9304] We still see enemy but we need to check if it close enogh to react
            (bind _ascharacter (cast `Character` _returnvalue_7))
            (bind _dead_2 (message `/Game/ShooterAI/Blueprints/BPI_ShooterAI.GetIsDead` _ascharacter))
            (if _dead_2
              (`BlackboardComponent.ClearValue` (`AIBlueprintHelperLibrary.GetBlackboard` null) "Enemy")
              (else
                (bind _distance (message `/Game/ShooterAI/Blueprints/BPI_ShooterAI.PawnGetMaxViewEnemyDistance` _returnvalue_2))
                (bind _returnvalue_8 (`self.K2_GetActorLocation` _ascharacter))
                (bind _returnvalue_9 (<= (`KismetMathLibrary.VSize` (- _returnvalue_8 (`self.K2_GetActorLocation` _returnvalue_2))) _distance))
                (if (not _returnvalue_9)
                  (bind _output_get (set `self.LastStimulusLocation` _returnvalue_8))
                  (`BlackboardComponent.SetValueAsVector` _returnvalue_5 "LastStimulusLocation" _output_get))
                (`BlackboardComponent.SetValueAsBool` _returnvalue_5 "WasTargetSeen" true)
                (`BlackboardComponent.SetValueAsBool` _returnvalue_5 "IsEnemyTooFarAway" (not _returnvalue_9))))
            (else
              (bind (_wasseen _location) (`self.GetLastSeenLocationOfTheObject` _returnvalue_6))
              (`BlackboardComponent.SetValueAsVector` _returnvalue_5 "LastSeenLocationOfTheTarget" _location)
              (`BlackboardComponent.ClearValue` _returnvalue_5 "Enemy"))))
        (:`Is Not Valid`
          ;[1 0.8786 0 1 10] Can see Enemy?
          (for _array_element_2 (`AIPerceptionComponent.GetPerceivedActors` (`self.AIPerception`) "/Script/AIModule.AISense_Sight")
            (bind _ascharacter_2 (cast `Character` _array_element_2))
            (bind (_value _returnvalue_10) (`BlueprintMapLibrary.Map_Find` (`self.Relationships`) (`GameplayStatics.GetObjectClass` _ascharacter_2)))
            (if _returnvalue_10
              (if (`|EnumEquality` _value "NewEnumerator0")
                (bind _dead_3 (message `/Game/ShooterAI/Blueprints/BPI_ShooterAI.GetIsDead` _array_element_2))
                (if (not _dead_3)
                  (bind _distance_2 (message `/Game/ShooterAI/Blueprints/BPI_ShooterAI.PawnGetMaxViewEnemyDistance` _returnvalue_4))
                  (bind _returnvalue_11 (`self.K2_GetActorLocation` _array_element_2))
                  (bind _returnvalue_12 (<= (`KismetMathLibrary.VSize` (- _returnvalue_11 (`self.K2_GetActorLocation` _returnvalue_4))) _distance_2))
                  (if (not _returnvalue_12)
                    (bind _output_get_2 (set `self.LastStimulusLocation` _returnvalue_11))
                    (`BlackboardComponent.SetValueAsVector` _returnvalue_3 "LastStimulusLocation" _output_get_2))
                  (`BlackboardComponent.SetValueAsObject` _returnvalue_3 "Enemy" _array_element_2)
                  (`BlackboardComponent.SetValueAsBool` _returnvalue_3 "WasTargetSeen" true)
                  (`BlackboardComponent.SetValueAsBool` _returnvalue_3 "IsEnemyTooFarAway" (not _returnvalue_12))
                  (break))))))))))

(fn `UserConstructionScript`)